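; Test actor that spawns procedural landscapes at runtime and shapes them from GPU-generated noise.
; Construction builds a dynamic material from Perlin and Voronoi settings, optionally baking immediately.
; DrawToRT renders that material to a render target and imports it as the landscape's heightmap.
; Debug keys spawn land, randomise the noise offset, refresh the material, shift the land, or spawn a timed grid of tiles without importing heightmaps.
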(event Custom|Create_new_land%28c%29
  (bind _returnvalue (Class|ProceuduralGameLandUtils|SpawnGameLand self (Variables|Default|GetTerrainMataterial) 1 8 8 127)) ; 7 15 31 63 127 255
  (bind _output_get (Variables|Landscape|SetLandscape2 _returnvalue))
  (Transformation|SetWorldScale3D (Variables|/Script/Engine.Actor|GetRootComponent _output_get) (Variables|Default|Getscale))
  (CallFunction|DrawtoRT))

(event Custom|RandomizeTerrainLocation%28x%29
  (Variables|Default|SetRandomOffset (Math|Random|RandomFloatinRange -5e+06 5e+06))
  (Rendering|Material|SetScalarParameterValue (Variables|Default|GetTerrainMat) "RandomOffset" (Variables|Default|GetRandomOffset) :!class /Script/Engine.MaterialInstanceDynamic)
  (CallFunction|DrawtoRT))

(event Custom|DrawToRT
  ;[1 1 1] Update Heightmap Render Target, apply Heightmap RT to Landscape, updating geometry/collisions
  (Rendering|DrawMaterialtoRenderTarget (Variables|Default|GetRT) (Variables|Default|GetTerrainMat))
  (Class|CyLandProxy|CyLandImportHeightmapfromRenderTargetmy (Variables|Landscape|GetLandscape2) (Variables|Default|GetRT) true))

(event Custom|AssignMat%28no%20effect%29
  (Variables|/Script/CyLand.CyLandProxy|SetCyLandMaterial (Variables|Landscape|GetLandscape2) (Variables|Default|GetTerrainMataterial)))

(event Custom|Update%20Mat%28fail%29
  (bind _landscape2 (Variables|Landscape|GetLandscape2))
  (Variables|/Script/CyLand.CyLandProxy|SetCyLandMaterial _landscape2 (Variables|Default|GetTerrainMataterial))
  (Class|ProceuduralGameLandUtils|NotifyMaterialUpdated _landscape2))

(event Custom|CrazyMegaTest
  (bind _crazydimen (Variables|Default|GetCrazyDimen))
  (bind _returnvalue (CallFunction|Now))
  (Utilities|FlowControl|Sequence
    (:then_0
      (for _index (range 0 _crazydimen)
        (for _index_2 (range 0 _crazydimen)
          (bind _returnvalue_2 (Class|ProceuduralGameLandUtils|SpawnGameLand self (Variables|Default|GetTerrainMataterial) 1 8 8 127)) ; 7 15 31 63 127 255
          (Variables|Landscape|SetLandscape2 _returnvalue_2)
          (if false ; jitter
            (CallFunction|RandomizeTerrainLocation(x)))
          (Transformation|AddWorldOffset (Variables|/Script/Engine.Actor|GetRootComponent (Variables|Landscape|GetLandscape2)) (Math|Vector|MakeVector (* (Math|Conversions|ToFloat(Integer) _index) (* (.x (Transformation|GetWorldScale (Variables|/Script/Engine.Actor|GetRootComponent (Variables|Landscape|GetLandscape2)))) 1016.0)) (* (Math|Conversions|ToFloat(Integer) _index_2) (* (.y (Transformation|GetWorldScale (Variables|/Script/Engine.Actor|GetRootComponent (Variables|Landscape|GetLandscape2)))) 1016.0)) 0.0) false false))))
    (:then_1
      (Development|PrintString "Time Elapsed Is:  ")
      (Development|PrintString (Utilities|String|Append (Utilities|String|ToString(Integer) (.hours (- (Math|DateTime|Now) _returnvalue))) "h, " (Utilities|String|ToString(Integer) (.minutes (- (Math|DateTime|Now) _returnvalue))) "m, " (Utilities|String|ToString(Integer) (.seconds (- (Math|DateTime|Now) _returnvalue))) "s") true true "(R=1.000000,G=0.107588,B=0.000000,A=1.000000)" 1e+06))))

(event EventBeginPlay)

(event Collision|EventActorBeginOverlap
  (params (OtherActor :type Actor%20Object%20Reference)))

(event EventTick
  (params (DeltaSeconds :type Float%20%28single-precision%29)))

(event Input|KeyboardEvents|C
  (params (Key :type Key%20Structure))
  (:Pressed
    (bind _returnvalue (Class|ProceuduralGameLandUtils|SpawnGameLand self (Variables|Default|GetTerrainMataterial) 1 8 8 127)) ; 7 15 31 63 127 255
    (bind _output_get (Variables|Landscape|SetLandscape2 _returnvalue))
    (Transformation|SetWorldScale3D (Variables|/Script/Engine.Actor|GetRootComponent _output_get) (Variables|Default|Getscale))
    (CallFunction|DrawtoRT)))

(event Input|KeyboardEvents|M
  (params (Key :type Key%20Structure))
  (bind _crazydimen (Variables|Default|GetCrazyDimen))
  (:Pressed
    (bind _returnvalue (CallFunction|Now))
    (Utilities|FlowControl|Sequence
      (:then_0
        (for _index (range 0 _crazydimen)
          (for _index_2 (range 0 _crazydimen)
            (bind _returnvalue_2 (Class|ProceuduralGameLandUtils|SpawnGameLand self (Variables|Default|GetTerrainMataterial) 1 8 8 127)) ; 7 15 31 63 127 255
            (Variables|Landscape|SetLandscape2 _returnvalue_2)
            (if false ; jitter
              (CallFunction|RandomizeTerrainLocation(x)))
            (Transformation|AddWorldOffset (Variables|/Script/Engine.Actor|GetRootComponent (Variables|Landscape|GetLandscape2)) (Math|Vector|MakeVector (* (Math|Conversions|ToFloat(Integer) _index) (* (.x (Transformation|GetWorldScale (Variables|/Script/Engine.Actor|GetRootComponent (Variables|Landscape|GetLandscape2)))) 1016.0)) (* (Math|Conversions|ToFloat(Integer) _index_2) (* (.y (Transformation|GetWorldScale (Variables|/Script/Engine.Actor|GetRootComponent (Variables|Landscape|GetLandscape2)))) 1016.0)) 0.0) false false))))
      (:then_1
        (Development|PrintString "Time Elapsed Is:  ")
        (Development|PrintString (Utilities|String|Append (Utilities|String|ToString(Integer) (.hours (- (Math|DateTime|Now) _returnvalue))) "h, " (Utilities|String|ToString(Integer) (.minutes (- (Math|DateTime|Now) _returnvalue))) "m, " (Utilities|String|ToString(Integer) (.seconds (- (Math|DateTime|Now) _returnvalue))) "s") true true "(R=1.000000,G=0.107588,B=0.000000,A=1.000000)" 1e+06)))))

(event Input|KeyboardEvents|X
  (params (Key :type Key%20Structure))
  (:Pressed
    (Variables|Default|SetRandomOffset (Math|Random|RandomFloatinRange -5e+06 5e+06))
    (Rendering|Material|SetScalarParameterValue (Variables|Default|GetTerrainMat) "RandomOffset" (Variables|Default|GetRandomOffset) :!class /Script/Engine.MaterialInstanceDynamic)
    (CallFunction|DrawtoRT)))

(event Input|KeyboardEvents|V
  (params (Key :type Key%20Structure))
  (bind _landscape2 (Variables|Landscape|GetLandscape2))
  (bind _rootcomponent (Variables|/Script/Engine.Actor|GetRootComponent _landscape2))
  (:Pressed
    (Transformation|AddWorldOffset _rootcomponent (Math|Vector|MakeVector (* (.x (Transformation|GetWorldScale _rootcomponent)) 1016.0) 0.0 0.0) false false)))

(event Input|KeyboardEvents|U
  (params (Key :type Key%20Structure))
  (bind _landscape2 (Variables|Landscape|GetLandscape2))
  (:Pressed
    (Variables|/Script/CyLand.CyLandProxy|SetCyLandMaterial _landscape2 (Variables|Default|GetTerrainMataterial))
    (Class|ProceuduralGameLandUtils|NotifyMaterialUpdated _landscape2)))

(fn ConstructionScript
  (CallFunction|AssignVariablestoTerrainConstructionDynamicMaterial)
  (if (Variables|Landscape|GetHotCookLandscape)
    (CallFunction|DrawtoRT)))

(fn AssignVariablestoTerrainConstructionDynamicMaterial
  (bind _returnvalue (Rendering|Material|CreateDynamicMaterialInstance "/Game/TerrainEditor/Materials/MI_TerrainConstructor.MI_TerrainConstructor" "None" :!class /Script/Engine.KismetMaterialLibrary))
  (bind _output_get (Variables|Default|SetTerrainMat _returnvalue))
  (Rendering|Material|SetScalarParameterValue _output_get "PerlinScale1" (Variables|Perlin1|GetPerlinScale1) :!class /Script/Engine.MaterialInstanceDynamic)
  (Rendering|Material|SetScalarParameterValue _output_get "PerlinContrast1" (Variables|Perlin1|GetPerlinContrast1) :!class /Script/Engine.MaterialInstanceDynamic)
  (Rendering|Material|SetScalarParameterValue _output_get "PerlinStrength1" (Variables|Perlin1|GetPerlinStrength1) :!class /Script/Engine.MaterialInstanceDynamic)
  (Rendering|Material|SetScalarParameterValue _output_get "Perlin1" (Variables|Perlin1|GetPerlin1) :!class /Script/Engine.MaterialInstanceDynamic)
  (Rendering|Material|SetScalarParameterValue _output_get "PerlinScale2" (Variables|Perlin2|GetPerlinScale2) :!class /Script/Engine.MaterialInstanceDynamic)
  (Rendering|Material|SetScalarParameterValue _output_get "PerlinContrast2" (Variables|Perlin2|GetPerlinContrast2) :!class /Script/Engine.MaterialInstanceDynamic)
  (Rendering|Material|SetScalarParameterValue _output_get "PerlinStrength2" (Variables|Perlin2|GetPerlinStrength2) :!class /Script/Engine.MaterialInstanceDynamic)
  (Rendering|Material|SetScalarParameterValue _output_get "Perlin2" (Variables|Perlin2|GetPerlin2) :!class /Script/Engine.MaterialInstanceDynamic)
  (Rendering|Material|SetScalarParameterValue _output_get "PerlinScale3" (Variables|Perlin3|GetPerlinScale3) :!class /Script/Engine.MaterialInstanceDynamic)
  (Rendering|Material|SetScalarParameterValue _output_get "PerlinContrast3" (Variables|Perlin3|GetPerlinContrast3) :!class /Script/Engine.MaterialInstanceDynamic)
  (Rendering|Material|SetScalarParameterValue _output_get "PerlinStrength3" (Variables|Perlin3|GetPerlinStrength3) :!class /Script/Engine.MaterialInstanceDynamic)
  (Rendering|Material|SetScalarParameterValue _output_get "Perlin3" (Variables|Perlin3|GetPerlin3) :!class /Script/Engine.MaterialInstanceDynamic)
  (Rendering|Material|SetScalarParameterValue (Variables|Default|GetTerrainMat) "OverallHeight" (Variables|Landscape|GetOverallHeight) :!class /Script/Engine.MaterialInstanceDynamic)
  (Rendering|Material|SetScalarParameterValue (Variables|Default|GetTerrainMat) "VoronoiContrast" (Variables|Voronoi|GetVoronoiContrast) :!class /Script/Engine.MaterialInstanceDynamic)
  (Rendering|Material|SetScalarParameterValue (Variables|Default|GetTerrainMat) "VoronoiStrength" (Variables|Voronoi|GetVoronoiStrength) :!class /Script/Engine.MaterialInstanceDynamic)
  (Rendering|Material|SetScalarParameterValue (Variables|Default|GetTerrainMat) "VoronoiScale" (Variables|Voronoi|GetVoronoiScale) :!class /Script/Engine.MaterialInstanceDynamic)
  (Rendering|Material|SetScalarParameterValue (Variables|Default|GetTerrainMat) "Voronoi" (Variables|Voronoi|GetVoronoi) :!class /Script/Engine.MaterialInstanceDynamic)
  (Rendering|Material|SetScalarParameterValue (Variables|Default|GetTerrainMat) "VoronoiBreakup" (Variables|Voronoi|GetVoronoiBreakup) :!class /Script/Engine.MaterialInstanceDynamic)
  (return))

(fn Now
  (return (Math|DateTime|Now)))